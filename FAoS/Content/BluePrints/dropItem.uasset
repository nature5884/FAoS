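; Dropped item pickup that homes in on the player and is collected on contact.
; Once the player overlaps the Sphere, Tick turns the item toward the player and moves it forward, turning faster when MoreNear is set.
; Player overlap with the StaticMesh broadcasts GetItem with the ItemType, sets IsHaveItem on MyCharacter, then destroys the item.
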(event `self.StaticMesh.OnComponentBeginOverlap`
  (params (OtherActor :type "Actor Object Reference") (OtherComp :type "PrimitiveComponent Object Reference") (OtherBodyIndex :type Integer) (bFromSweep :type Boolean) (SweepResult :type "HitResult Structure (by ref)"))
  (bind _returnvalue (`GameplayStatics.GetPlayerPawn` 0))
  (if (== OtherActor _returnvalue)
    (`self.GetItem` (`self.itemType`))
    (bind _asmy_character (cast `/Game/BluePrints/MyCharacter` _returnvalue))
    (set `/Game/BluePrints/MyCharacter.isHaveItem` true _asmy_character)
    (`self.K2_DestroyActor`)))

(event `self.Sphere.OnComponentBeginOverlap`
  (params (OtherActor :type "Actor Object Reference") (OtherComp :type "PrimitiveComponent Object Reference") (OtherBodyIndex :type Integer) (bFromSweep :type Boolean) (SweepResult :type "HitResult Structure (by ref)"))
  (if (== OtherActor (`GameplayStatics.GetPlayerPawn` 0))
    (set `self.nearPlayer` true)))

(event `self.ReceiveTick`
  (params (DeltaSeconds :type "Float (single-precision)"))
  (bind _returnvalue (`self.K2_GetActorRotation`))
  (if (`self.nearPlayer`)
    (if (`self.moreNear`)
      (set `self.interpSpeed` 10.0))
    (`SceneComponent.K2_SetWorldRotation` (`self.DefaultSceneRoot`) (`KismetMathLibrary.RInterpTo` _returnvalue (`KismetMathLibrary.FindLookAtRotation` (`self.K2_GetActorLocation`) (`self.K2_GetActorLocation` (`GameplayStatics.GetPlayerPawn` 0))) DeltaSeconds (`self.interpSpeed`)) false false)
    (`self.K2_AddActorWorldOffset` (* (`KismetMathLibrary.GetForwardVector` _returnvalue) (* DeltaSeconds (`self.speed`))))))

(event `self.ReceiveBeginPlay`
  (set `self.interpSpeed` 5.0))

(fn `UserConstructionScript`)