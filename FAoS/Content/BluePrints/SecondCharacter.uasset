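; SecondCharacter is a player-controlled Blueprint that provides basic movement and mouse look through input axis events.
; MoveForword and MoveInfluence feed movement input along forward and right vectors built from control rotation yaw only, keeping motion on the horizontal plane.
; MouseTurn and MouseLookUp pass their axis values straight to controller yaw and pitch.
; BeginPlay, Tick, overlap and the construction script are empty.
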(event `InputAxis|MoveForword`
  (params (AxisValue :type "Float (single-precision)"))
  (`self.AddMovementInput` (`KismetMathLibrary.GetForwardVector` (`KismetMathLibrary.MakeRotator` 0.0 0.0 (.yaw (`self.GetControlRotation`)))) AxisValue))

(event `InputAxis|MoveInfluence`
  (params (AxisValue :type "Float (single-precision)"))
  (`self.AddMovementInput` (`KismetMathLibrary.GetRightVector` (`KismetMathLibrary.MakeRotator` 0.0 0.0 (.yaw (`self.GetControlRotation`)))) AxisValue))

(event `InputAxis|MouseTurn`
  (params (AxisValue :type "Float (single-precision)"))
  (`self.AddControllerYawInput` AxisValue))

(event `InputAxis|MouseLookUp`
  (params (AxisValue :type "Float (single-precision)"))
  (`self.AddControllerPitchInput` AxisValue))

(fn `UserConstructionScript`)