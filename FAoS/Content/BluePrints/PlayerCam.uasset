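; PlayerCam is a camera actor that trails the player pawn in X and Y within level bounds.
; BeginPlay caches the WaveMgr and reads the bounds from a CameraLimitPos actor and its Limit component.
; Each Tick, CameraMove offsets the camera by one fifteenth of the Arrow-to-player gap, a frame-rate-dependent easing gated per direction by those bounds.
; Tick also hides the camera component in game unless WaveMgr.IsPlayerCam is set.
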(event `self.ReceiveBeginPlay`
  (bind _outactors (`GameplayStatics.GetAllActorsOfClass` "/Game/BluePrints/BattleActors/WaveMgr.WaveMgr_C"))
  (set `self.waveMgr` (`KismetArrayLibrary.Array_Get` _outactors))
  (bind _outactors_2 (`GameplayStatics.GetAllActorsOfClass` "/Game/BluePrints/CameraLimitPos.CameraLimitPos_C"))
  (bind _item (`KismetArrayLibrary.Array_Get` _outactors_2))
  (bind (_returnvalue_x _returnvalue_y) (`KismetMathLibrary.BreakVector` (`self.K2_GetActorLocation` _item)))
  (set `self.MIN_X` _returnvalue_x)
  (set `self.MIN_Y` _returnvalue_y)
  (bind (_returnvalue_x_2 _returnvalue_y_2) (`KismetMathLibrary.BreakVector` (`SceneComponent.K2_GetComponentLocation` (`/Game/BluePrints/CameraLimitPos.Limit` _item))))
  (set `self.MAX_X` _returnvalue_x_2)
  (set `self.MAX_Y` _returnvalue_y_2))

(event `self.ReceiveTick`
  (params (DeltaSeconds :type "Float (single-precision)"))
  (bind _cameracomponent (`self.CameraComponent`))
  (bind (_returnvalue_x _returnvalue_y) (`KismetMathLibrary.BreakVector` (`SceneComponent.K2_GetComponentLocation` _cameracomponent)))
  (bind (_returnvalue_x_2 _returnvalue_y_2) (`KismetMathLibrary.BreakVector` (- (`SceneComponent.K2_GetComponentLocation` (`self.Arrow`)) (`self.K2_GetActorLocation` (`GameplayStatics.GetPlayerPawn` 0)))))
  (`|ExecutionSequence`
    (:`then_0`
      (`|ExecutionSequence`
        (:`then_0`
          (if (> _returnvalue_x_2 0.0)
            (if (> _returnvalue_x (`self.MAX_X`))
              (`SceneComponent.K2_AddWorldOffset` _cameracomponent (`KismetMathLibrary.MakeVector` (/ _returnvalue_x_2 -15.0)) false false :!label _label))
            (elif (< _returnvalue_x (`self.MIN_X`))
              (goto _label))))
        (:`then_1`
          (if (> _returnvalue_y_2 0.0)
            (if (> _returnvalue_y (`self.MIN_Y`))
              (`SceneComponent.K2_AddWorldOffset` _cameracomponent (`KismetMathLibrary.MakeVector` 0.0 (/ _returnvalue_y_2 -15.0)) false false :!label _label_2))
            (elif (< _returnvalue_y (`self.MAX_Y`))
              (goto _label_2))))))
    (:`then_1`
      (`SceneComponent.SetHiddenInGame` (`self.CameraComponent`) (not (`/Game/BluePrints/BattleActors/WaveMgr.isPlayerCam` (`self.waveMgr`))) false))))

(fn `UserConstructionScript`)