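; Spawner for three types of Sozai (material) actors that tracks the remaining stock of each in SozaiTotalNum.
; Tick prints the counts and calls Spawn, which randomly picks an in-stock type, spawns a half-scale Sozais after a one-second Delay and decrements its count.
; SozaiDeath's SozaiReverse event, bound at BeginPlay, returns stock, while Sozais' SozaiFluctuation, rebound every Tick, also decrements it.
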(event `素材戻ってきたよ`
  (params (NewParam :type "/Game/BluePrints/testElem Enum"))
  (bind _returnvalue (`KismetMathLibrary.Conv_ByteToInt` NewParam))
  (bind _sozaitotalnum (`self.sozaiTotalNum`))
  (set `self.getSozaiReverseNum` (`KismetArrayLibrary.Array_Get` _sozaitotalnum _returnvalue))
  (`KismetArrayLibrary.Array_Set` _sozaitotalnum _returnvalue (+ (`self.getSozaiReverseNum`) 1)))

(event `self.ReceiveBeginPlay`
  (bind _outactors (`GameplayStatics.GetAllActorsOfClass` "/Game/BluePrints/sozaiDeath.sozaiDeath_C"))
  (add `/Game/BluePrints/sozaiDeath.SozaiReverse` _outactors (delegate `素材戻ってきたよ`)))

(event `素材減らす`
  (params (NewParam :type Byte))
  (bind _returnvalue (`KismetMathLibrary.Conv_ByteToInt` NewParam))
  (bind _getsozainum (`self.getSozaiNum`))
  (bind _sozaitotalnum (`self.sozaiTotalNum`))
  (set `self.getSozaiNum` (`KismetArrayLibrary.Array_Get` _sozaitotalnum _returnvalue))
  (if (!= _getsozainum 0)
    (`KismetArrayLibrary.Array_Set` _sozaitotalnum _returnvalue (- _getsozainum 1))))

(event `self.ReceiveTick`
  (params (DeltaSeconds :type "Float (single-precision)"))
  (`|ExecutionSequence`
    (:`then_0`
      (for (_array_element _array_index) (`self.sozaiTotalNum`)
        (switch `int` _array_index
          (:`0`
            (bind _returnvalue (`KismetStringLibrary.Conv_ByteToString` _array_element))
            (`KismetSystemLibrary.PrintString` _returnvalue true true (struct :`R` 1.0 :`A` 1.0)))
          (:`1`
            (`KismetSystemLibrary.PrintString` _returnvalue true true (struct :`G` 1.0 :`A` 1.0)))
          (:`2`
            (`KismetSystemLibrary.PrintString` _returnvalue true true (struct :`B` 1.0 :`A` 1.0)))))
      (`self.Spawn`))
    (:`then_1`
      (bind _outactors (`GameplayStatics.GetAllActorsOfClass` "/Game/BluePrints/Sozais.Sozais_C"))
      (add `/Game/BluePrints/Sozais.SozaiFluctuation` _outactors (delegate `素材減らす`)))))

(event `Spawn`
  (bind (_returnvalue_location _returnvalue_rotation) (`KismetMathLibrary.BreakTransform` (`self.GetTransform`)))
  (bind _gettype (`self.getType`))
  (for (_array_element _array_index) (`self.sozaiTotalNum`)
    (if (and (!= _array_element 0) (== _array_index (`KismetMathLibrary.RandomIntegerInRange` 0 2)))
      (set `self.getType` (`KismetArrayLibrary.Array_Get` (`self.MyType`) _array_index))
      (`KismetSystemLibrary.Delay` 1.0)
      (`|SpawnActorFromClass` "/Game/BluePrints/Sozais.Sozais_C" (`KismetMathLibrary.MakeTransform` _returnvalue_location _returnvalue_rotation (0.5 0.5 0.5)) "Undefined" "OverrideRootScale" null _gettype)
      (`self.素材減らす` _gettype)
      (break))))

(fn `UserConstructionScript`)