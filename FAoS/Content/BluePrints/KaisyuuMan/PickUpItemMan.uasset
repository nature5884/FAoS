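; PickUpItemMan is a collector actor that picks up dropped items it touches.
; When its capsule overlaps an actor whose class is exactly DropItem, it appends the item's MyType to DropElements and ItemType to DropSlimeTypes, then destroys the item.
; PopDropData returns both parallel arrays to callers but, despite its name, does not clear them.
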(event `self.ReceiveBeginPlay`)

(event `self.ReceiveActorBeginOverlap`
  (params (OtherActor :type "Actor Object Reference")))

(event `self.CapsuleComponent.OnComponentBeginOverlap`
  (params (OtherActor :type "Actor Object Reference") (OtherComp :type "PrimitiveComponent Object Reference") (OtherBodyIndex :type Integer) (bFromSweep :type Boolean) (SweepResult :type "HitResult Structure (by ref)"))
  (if (== (`GameplayStatics.GetObjectClass` OtherActor) "/Game/BluePrints/dropItem.dropItem_C")
    (bind _asdrop_item (cast `/Game/BluePrints/dropItem` OtherActor))
    (`KismetArrayLibrary.Array_Add` (`self.drop_Elements`) (`/Game/BluePrints/dropItem.MyType` _asdrop_item))
    (`KismetArrayLibrary.Array_Add` (`self.drop_SlimeTypes`) (`/Game/BluePrints/dropItem.itemType` _asdrop_item))
    (`self.K2_DestroyActor` OtherActor)))

(fn `PopDropData`
  (returns (drop_Elements :type "Array of /Game/BluePrints/sozai/testElem Enum") (drop_SlimeTypes :type "Array of /Game/BluePrints/BattleActors/SlimeType Enum"))
  (return (`self.drop_Elements`) (`self.drop_SlimeTypes`)))

(fn `UserConstructionScript`)