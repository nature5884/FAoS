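; Sozais is a rock-paper-scissors item actor that shows one of three hand types and can be destroyed by the player.
; On BeginPlay it sets its mesh material from MyType (グー, チョキ or パー) and binds to MyCharacter's SozaiDestroy dispatcher.
; When that dispatcher fires, the actor destroys itself only if it is the character's current Target.
; The replication callback for sozaisTotalNum is empty.
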(event `self.ReceiveBeginPlay`
  (bind _staticmeshcomponent (`self.StaticMeshComponent`))
  (bind _asmy_character (cast `/Game/BluePrints/MyCharacter` (`GameplayStatics.GetPlayerPawn` 0))
    (:`then`
      (add `/Game/BluePrints/MyCharacter.SozaiDestroy` _asmy_character (delegate `Destroy`)))
    (:`CastFailed`
      _))
  (switch `/Game/BluePrints/testElem` (`self.MyType`)
    (:`NewEnumerator0`
      (`PrimitiveComponent.SetMaterial` _staticmeshcomponent 0 "/Game/Texture/グー.グー"))
    (:`NewEnumerator1`
      (`PrimitiveComponent.SetMaterial` _staticmeshcomponent 0 "/Game/Texture/チョキ.チョキ"))
    (:`NewEnumerator2`
      (`PrimitiveComponent.SetMaterial` _staticmeshcomponent 0 "/Game/Texture/パー.パー"))))

(event `Destroy`
  (if (== (`/Game/BluePrints/MyCharacter.Target` (stale `self.ReceiveBeginPlay` _asmy_character)) self)
    (`self.K2_DestroyActor`)))

(fn `OnRep_sozaisTotalNum`)

(fn `UserConstructionScript`)