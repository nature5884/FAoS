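; Player character that walks, jumps, and carries "sozai" material items to throw into a SlimeCreater.
; CaptureBox overlaps lock one target through a DoOnce; E alternates grab and throw via a MultiGate, with Tick pinning the held item to CapturePoint.
; Throws call slime creation with the item's type when the creater allows, otherwise release it with an impulse.
; K toggles a movement-locking camera zoom gated by a Test actor, during which C calls a capture-screen change.
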(event `Key|SpaceBar`
  (params (Key :type "Key Structure" :default "AnyKey"))
  (:`Pressed`
    (`self.Jump`))
  (:`Released`
    (`self.StopJumping`)))

(event `Key|C`
  (params (Key :type "Key Structure" :default "AnyKey"))
  (:`Pressed`
    (if (`self.camZoomNow`)
      (`self.CaptureScreenChange`))))

(event `self.ReceiveBeginPlay`
  (bind _outactors (`GameplayStatics.GetAllActorsOfClass` "/Game/BluePrints/SlimeCreater.SlimeCreater_C"))
  (set `self.SlimeCreater` (`KismetArrayLibrary.Array_Get` _outactors)))

(event `InputAxis|MoveForword` :overrideparent false
  (params (AxisValue :type "Float (single-precision)"))
  (`self.AddMovementInput` (`KismetMathLibrary.GetForwardVector` (`KismetMathLibrary.MakeRotator` 0.0 0.0 (.yaw (`self.GetControlRotation`)))) AxisValue))

(event `InputAxis|MoveInfluence` :overrideparent false
  (params (AxisValue :type "Float (single-precision)"))
  (`self.AddMovementInput` (`KismetMathLibrary.GetRightVector` (`KismetMathLibrary.MakeRotator` 0.0 0.0 (.yaw (`self.GetControlRotation`)))) AxisValue))

(event `Key|K`
  (params (Key :type "Key Structure" :default "AnyKey"))
  (bind _camera (`self.Camera`))
  (:`Pressed`
    (bind _outactors (`GameplayStatics.GetAllActorsOfClass` "/Game/BluePrints/test.test_C"))
    (if (`/Game/BluePrints/test.isComZoom` (`KismetArrayLibrary.Array_Get` _outactors))
      (if (`self.camZoomNow`)
        (`KismetSystemLibrary.MoveComponentTo` _camera (.location (`SceneComponent.GetRelativeTransform` (`self.Arrow2`))) (.rotation (`SceneComponent.GetRelativeTransform` (`self.Arrow2`))) false false 1.0)
        (set `self.camZoomNow` false)
        (`CharacterMovementComponent.SetMovementMode` (`self.CharacterMovement`) "MOVE_Walking" 0)
        (else
          (`CharacterMovementComponent.DisableMovement` (`self.CharacterMovement`))
          (set `self.camZoomNow` true)
          (`KismetSystemLibrary.MoveComponentTo` _camera (.location (`SceneComponent.GetRelativeTransform` (`self.Arrow1`))) (struct) false false 1.0))))))

(event `InputAxis|MouseTurn`
  (params (AxisValue :type "Float (single-precision)")))

(event `InputAxis|MouseLookUp`
  (params (AxisValue :type "Float (single-precision)")))

(event `self.ReceiveTick`
  (params (DeltaSeconds :type "Float (single-precision)"))
  (bind _sozaitarget (`self.sozaiTarget`))
  (bind (_returnvalue_location _returnvalue_rotation) (`KismetMathLibrary.BreakTransform` (`SceneComponent.K2_GetComponentToWorld` (`self.capturePoint`))))
  (`|ExecutionSequence`
    (:`then_0`
      (if (`self.camZoomNow`)
        (`SceneComponent.K2_SetWorldRotation` (`self.CapsuleComponent`) (.rotation (`SceneComponent.GetRelativeTransform` (`self.Arrow1`))) false false)))
    (:`then_1`
      (switch `int` (`self.captureMode`)
        (:`0`
          (if (`self.isPossess`)
            (`PrimitiveComponent.SetSimulatePhysics` _sozaitarget false)
            (`SceneComponent.K2_SetWorldTransform` _sozaitarget (`KismetMathLibrary.MakeTransform` _returnvalue_location _returnvalue_rotation (`SceneComponent.K2_GetComponentScale` _sozaitarget)) false false)))
        (:`1`
          (`PrimitiveComponent.SetSimulatePhysics` _sozaitarget true)
          (set `self.captureMode` -1))))))

(event `self.CaptureBox.OnComponentBeginOverlap`
  (params (OtherActor :type "Actor Object Reference") (OtherComp :type "PrimitiveComponent Object Reference") (OtherBodyIndex :type Integer) (bFromSweep :type Boolean) (SweepResult :type "HitResult Structure (by ref)"))
  (switch `int` (`self.captureMode`)
    (:`Default`
      _)
    (:`1`
      _))
  (if (`ActorComponent.ComponentHasTag` OtherComp "sozai")
    (`/Engine/EditorBlueprintResources/StandardMacros.DoOnce` false :!label _label
      (:`Completed`
        (set `self.Target` OtherActor)
        (set `self.sozaiTarget` OtherComp)
        (bind _assozais (cast `/Game/BluePrints/sozai/Sozais` OtherActor))
        (set `self.sozaisType` (`/Game/BluePrints/sozai/Sozais.MyStruct` _assozais))
        (set `self.isCapture` true)))))

(event `Key|E`
  (params (Key :type "Key Structure" :default "AnyKey"))
  (bind _sozaitarget (`self.sozaiTarget`))
  (bind _slimecreater (`self.SlimeCreater`))
  (bind (_returnvalue_location _returnvalue_rotation) (`KismetMathLibrary.BreakTransform` (`SceneComponent.GetRelativeTransform` _sozaitarget)))
  (:`Pressed`
    (if (`self.isCapture`)
      (`|MultiGate` false :!label _label_2
        (:`Out 0`
          (set `self.captureMode` 0)
          (set `self.isPossess` true)
          (`KismetSystemLibrary.MoveComponentTo` _sozaitarget (`SceneComponent.K2_GetComponentLocation` (`self.capturePoint`)) (struct) false false 0.1)
          (`PrimitiveComponent.SetCollisionEnabled` _sozaitarget "NoCollision"))
        (:`Out 1`
          (if (`/Game/BluePrints/SlimeCreater.canThrow` _slimecreater)
            (set `self.isPossess` false)
            (`KismetSystemLibrary.MoveComponentTo` _sozaitarget (`SceneComponent.K2_GetComponentLocation` (`/Game/BluePrints/SlimeCreater.Arrow` _slimecreater)) _returnvalue_rotation false false 0.5)
            (`self.SozaiDestroy`)
            (`self.SlimeCreate` (`self.sozaisType`))
            (set `self.captureMode` 1)
            (else
              (set `self.captureMode` 1)
              (`PrimitiveComponent.SetCollisionEnabled` _sozaitarget "QueryAndPhysics")
              (set `self.isPossess` false)
              (`PrimitiveComponent.AddImpulse` _sozaitarget (100.0 0.0 0.0) "None" false)))
          (`|ExecutionSequence`
            (:`then_0`
              (goto _label_2 :!via `Reset`))))))))

(event `self.CaptureBox.OnComponentEndOverlap`
  (params (OtherActor :type "Actor Object Reference") (OtherComp :type "PrimitiveComponent Object Reference") (OtherBodyIndex :type Integer))
  (switch `int` (`self.captureMode`)
    (:`Default`
      _)
    (:`1`
      _))
  (if (`self.isCapture`)
    (set `self.isCapture` false)
    (goto _label :!via `Reset`)))

(fn `UserConstructionScript`)