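; Sozais is a material pickup actor (sozai) whose look depends on its type: rock, paper, scissors, feather or zombie.
; On BeginPlay it binds its Destroy event to the player character's SozaiDestroy dispatcher and turns off mesh physics, provided the cast to MyCharacter succeeds.
; It then sets the material by type, also swapping the mesh for zombies.
; When Destroy fires, it removes itself only if it is the character's current Target.
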(event `self.ReceiveBeginPlay`
  (bind _staticmeshcomponent (`self.StaticMeshComponent`))
  (bind _staticmeshcomponent_2 (`self.StaticMeshComponent`))
  (bind _asmy_character (cast `/Game/BluePrints/MyCharacter` (`GameplayStatics.GetPlayerPawn` 0))
    (:`then`
      (add `/Game/BluePrints/MyCharacter.SozaiDestroy` _asmy_character (delegate `Destroy`))
      (`PrimitiveComponent.SetSimulatePhysics` (`self.StaticMeshComponent`) false))
    (:`CastFailed`
      _))
  (switch `/Game/BluePrints/sozai/testElem` (`self.MyType`)
    (:`NewEnumerator0`
      (`PrimitiveComponent.SetMaterial` _staticmeshcomponent 0 "/Game/Texture/グー.グー"))
    (:`NewEnumerator1`
      (`PrimitiveComponent.SetMaterial` _staticmeshcomponent 0 "/Game/Texture/チョキ.チョキ"))
    (:`NewEnumerator2`
      (`PrimitiveComponent.SetMaterial` _staticmeshcomponent 0 "/Game/Texture/パー.パー"))
    (:`NewEnumerator3`
      (`PrimitiveComponent.SetMaterial` _staticmeshcomponent 0 "/Game/Model/kabe.kabe"))
    (:`NewEnumerator5`
      (`StaticMeshComponent.SetStaticMesh` _staticmeshcomponent_2 "/Game/Model/Item/Zombie/zombie_core.zombie_core")
      (`PrimitiveComponent.SetMaterial` _staticmeshcomponent_2 0 "/Game/Model/Item/Zombie/zombie_material_1.zombie_material_1")
      (`PrimitiveComponent.SetMaterial` _staticmeshcomponent_2 1 "/Game/Model/Item/Zombie/zombie_material_2.zombie_material_2")
      (`PrimitiveComponent.SetMaterial` _staticmeshcomponent_2 2 "/Game/Model/Item/Zombie/zombie_material_3.zombie_material_3"))))

(event `Destroy`
  (if (== (`/Game/BluePrints/MyCharacter.Target` (stale `self.ReceiveBeginPlay` _asmy_character)) self)
    (`self.K2_DestroyActor`)))

(fn `OnRep_sozaisTotalNum`)

(fn `UserConstructionScript`)