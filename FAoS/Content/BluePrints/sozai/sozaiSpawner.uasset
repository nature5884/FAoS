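; Material (sozai) spawner that tracks a stock count per material type and spawns Sozais actors at its own transform from that stock.
; Construction script fills the type list from an enum and pads the count array to match.
; Tick attempts a random in-stock pick, looks up its ItemType row, then spawns after a delay and decrements stock.
; DropItem and SozaiDeath dispatchers add stock, while Sozais fluctuation events, rebound every Tick, subtract it.
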(event `GetItem`
  (params (NewParam :type "/Game/BluePrints/sozai/testElem Enum"))
  (bind _sozaitotalnum (`self.sozaiTotalNum`))
  (for (_array_element _array_index) (`self.MyType`)
    (if (`KismetStringLibrary.EqualEqual_StrStr` (`|GetEnumeratorNameAsString` NewParam) (`|GetEnumeratorNameAsString` _array_element))
      (`KismetArrayLibrary.Array_Set` _sozaitotalnum _array_index (+ (`KismetArrayLibrary.Array_Get` _sozaitotalnum _array_index) 1))
      (break))))

(event `素材戻ってきたよ`
  (params (NewParam :type "/Game/BluePrints/sozai/testElem Enum"))
  (bind _returnvalue (`KismetMathLibrary.Conv_ByteToInt` NewParam))
  (bind _sozaitotalnum (`self.sozaiTotalNum`))
  (set `self.getSozaiReverseNum` (`KismetArrayLibrary.Array_Get` _sozaitotalnum _returnvalue))
  (`KismetArrayLibrary.Array_Set` _sozaitotalnum _returnvalue (+ (`self.getSozaiReverseNum`) 1)))

(event `self.ReceiveBeginPlay`
  (bind _outactors (`GameplayStatics.GetAllActorsOfClass` "/Game/BluePrints/sozai/sozaiDeath.sozaiDeath_C"))
  (add `/Game/BluePrints/sozai/sozaiDeath.SozaiReverse` _outactors (delegate `素材戻ってきたよ`))
  (bind _outactors_2 (`GameplayStatics.GetAllActorsOfClass` "/Game/BluePrints/dropItem.dropItem_C"))
  (add `/Game/BluePrints/dropItem.GetItem` _outactors_2 (delegate `GetItem`))
  (`KismetSystemLibrary.PrintString` "Hello" true true (struct :`R` 0.333636 :`G` 1.0 :`A` 1.0)))

(event `素材減らす`
  (params (NewParam :type Byte))
  (bind _returnvalue (`KismetMathLibrary.Conv_ByteToInt` NewParam))
  (bind _getsozainum (`self.getSozaiNum`))
  (bind _sozaitotalnum (`self.sozaiTotalNum`))
  (set `self.getSozaiNum` (`KismetArrayLibrary.Array_Get` _sozaitotalnum _returnvalue))
  (if (!= _getsozainum 0)
    (`KismetArrayLibrary.Array_Set` _sozaitotalnum _returnvalue (- _getsozainum 1))))

(event `self.ReceiveTick`
  (params (DeltaSeconds :type "Float (single-precision)"))
  (`|ExecutionSequence`
    (:`then_0`
      (`self.Spawn`))
    (:`then_1`
      (bind _outactors (`GameplayStatics.GetAllActorsOfClass` "/Game/BluePrints/sozai/Sozais.Sozais_C"))
      (add `/Game/BluePrints/sozai/Sozais.SozaiFluctuation` _outactors (delegate `素材減らす`)))))

(event `Spawn`
  (bind (_returnvalue_location _returnvalue_rotation) (`KismetMathLibrary.BreakTransform` (`self.GetTransform`)))
  (bind _sozaitotalnum (`self.sozaiTotalNum`))
  (bind _gettype (`self.getType`))
  (for (_array_element _array_index) _sozaitotalnum
    (if (and (!= _array_element 0) (== _array_index (`KismetMathLibrary.RandomIntegerInRange` 0 (`KismetArrayLibrary.Array_Length` _sozaitotalnum))))
      (set `self.getType` (`KismetArrayLibrary.Array_Get` (`self.MyType`) _array_index))
      (bind _returnvalue (`|GetDataTableRow` "/Game/BluePrints/sozai/ItemType.ItemType" (`KismetStringLibrary.Conv_StringToName` (`|GetEnumeratorNameAsString` _gettype)))
        (:`then`
          (`KismetSystemLibrary.Delay` 3.0)
          (bind (`_生成数` `_タイプ`) (break `/Game/BluePrints/sozai/ItemTypeStructure` _returnvalue))
          (`|SpawnActorFromClass` "/Game/BluePrints/sozai/Sozais.Sozais_C" (`KismetMathLibrary.MakeTransform` _returnvalue_location _returnvalue_rotation (1.0 1.0 1.0)) "Undefined" "OverrideRootScale" null `_タイプ` `_生成数` _returnvalue)
          (`self.素材減らす` _gettype)
          (break))
        (:`RowNotFound`
          (`KismetSystemLibrary.PrintString` "RowNotFownd"))))))

(fn `UserConstructionScript`
  (bind _sozaitotalnum (`self.sozaiTotalNum`))
  (bind _enumvalue (foreach `/Game/BluePrints/sozai/testElem`)
    (:`LoopBody`
      (`KismetArrayLibrary.Array_Add` (`self.MyType`) _enumvalue))
    (:`then`
      (for _ (range (+ (`KismetArrayLibrary.Array_Length` _sozaitotalnum) 1) (+ (`KismetArrayLibrary.Array_Length` (`self.MyType`)) 1))
        (`KismetArrayLibrary.Array_Add` _sozaitotalnum)))))