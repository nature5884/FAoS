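; Behavior Tree decorator for battle actors that gates a branch on how close the pawn is to its move destination.
; It passes when the distance from the pawn's location to the destination vector stored in the Blackboard is at most UnderValue.
; Slimes and pawns that are not BattleActors always fail the check.
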(fn `PerformConditionCheckAI`
  (params (OwnerController :type "AIController Object Reference") (ControlledPawn :type "Pawn Object Reference"))
  (returns (ReturnValue :type Boolean))
  (bind _asbattle_actor (cast `/Game/BluePrints/BattleActors/BattleActor` ControlledPawn)
    (:`then`
      (if (`/Game/BluePrints/BattleActors/BattleActor.isSlime` _asbattle_actor)
        _
        (else
          (return (<= (`KismetMathLibrary.VSize` (- (`BTFunctionLibrary.GetBlackboardValueAsVector` (`self.BBKey_moveDistination`)) (`Actor.K2_GetActorLocation` ControlledPawn))) (`self.underValue`))))))
    (:`CastFailed`
      _))
  (return false))