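; Enemy spawn manager actor that creates a battle wave's enemies from a data table.
; SpawnEnemys reads the SpawnTable row named by wave number, treats its ten columns as per-type counts, and returns the next wave number and enemy count.
; Each enemy spawns as an AI BattleActor along an X-offset line, receiving status from EnemyStateTable by row index, plus mesh and AnimBP from type-indexed arrays.
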(event EventBeginPlay)

(event EventActorBeginOverlap
  (params (OtherActor :type Actor%20Object%20Reference)))

(event EventTick
  (params (DeltaSeconds :type Float%20%28single-precision%29)))

(fn ConstructionScript)

(fn SpawnEnemys
  (params (waveNo :type Integer))
  (bind _returnvalue (Utilities|GetDataTableRow "/Game/BluePrints/BattleActors/SpawnTable.SpawnTable" (Utilities|String|StringToName (Utilities|String|ToString(Integer) waveNo)))
    (:then
      (for (_array_element _array_index) (Utilities|Array|MakeArray (.Enemy1 (Utilities|Struct|BreakStr_SpawnTable _returnvalue)) (.Enemy2 (Utilities|Struct|BreakStr_SpawnTable _returnvalue)) (.Enemy3 (Utilities|Struct|BreakStr_SpawnTable _returnvalue)) (.Enemy4 (Utilities|Struct|BreakStr_SpawnTable _returnvalue)) (.Enemy5 (Utilities|Struct|BreakStr_SpawnTable _returnvalue)) (.Enemy6 (Utilities|Struct|BreakStr_SpawnTable _returnvalue)) (.Enemy7 (Utilities|Struct|BreakStr_SpawnTable _returnvalue)) (.Enemy8 (Utilities|Struct|BreakStr_SpawnTable _returnvalue)) (.Enemy9 (Utilities|Struct|BreakStr_SpawnTable _returnvalue)) (.Enemy10 (Utilities|Struct|BreakStr_SpawnTable _returnvalue)))
        (if (!= _array_element 0)
          (for _index (range 1 _array_element)
            (|敵の生成 _array_index)
            (Math|Integer|IncrementInt (LocalVariables|GetspawnEnemyCnt)))))
      (Variables|Default|Setoffset 50)
      (bind _result (Math|Integer|IncrementInt waveNo)
        (:%20%20
          (return _result (LocalVariables|GetspawnEnemyCnt)))))
    (:RowNotFound
      (Development|PrintString "DTRowが見つからない")
      (return waveNo 0))))