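; Battle character shared by slimes and enemies, configured from a status struct with HP, movement, rock-paper-scissors element material and slime-type mesh.
; PawnSensing targets opposing-tagged actors, and Tick clears targets on death or when a sighting countdown expires.
; SetTargetActor searches overlaps, deferring already-fighting candidates via Blackboard flags.
; Attack only raises a flag; Damage applies element multipliers, destroys dead actors and decrements WaveMgr's enemy count.
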(event OnComponentBeginOverlap(Box)
  (params (OtherActor :type Actor%20Object%20Reference) (OtherComp :type Primitive%20Component%20Object%20Reference) (OtherBodyIndex :type Integer) (bFromSweep :type Boolean) (SweepResult :type Hit%20Result%20Structure%20%28by%20ref%29)))

(event OnSeePawn(PawnSensing)
  (params (Pawn :type Pawn%20Object%20Reference))
  (if (== (Variables|Default|GettargetActor) 0)
    (bind _asbattle_actor (Utilities|Casting|CastToBattleActor Pawn))
    (if (Variables|Default|GetisSlime)
      (if (Components|ComponentHasTag (Variables|/Script/Engine.Character|GetCapsuleComponent _asbattle_actor) "Enemy")
        (Variables|Default|SettargetActor _asbattle_actor :!label _label))
      (elif (Components|ComponentHasTag (Variables|/Script/Engine.Character|GetCapsuleComponent _asbattle_actor) "Slime")
        (goto _label)))
    (else
      (Variables|Default|SetmiusinattaCnt 300))))

(event EventBeginPlay
  (Variables|Default|SettargetActor 0))

(event EventActorBeginOverlap
  (params (OtherActor :type Actor%20Object%20Reference)))

(event EventTick
  (params (DeltaSeconds :type Float%20%28single-precision%29))
  (Utilities|FlowControl|Sequence
    (:then_0
      (if (>= (Variables|Default|GetmiusinattaCnt) 1)
        (Math|Integer|DecrementInt (Variables|Default|GetmiusinattaCnt))
        (else
          (Variables|Default|SettargetActor (Variables|Default|GetnullActor)))))
    (:then_1
      (bind _asbattle_actor (Utilities|Casting|CastToBattleActor (Variables|Default|GettargetActor)))
      (if (<= (Variables|BattleActor_C|GetHP _asbattle_actor) 0.0)
        (Variables|Default|SettargetActor (Variables|Default|GetnullActor))))))

(fn ConstructionScript)

(fn Attack
  (Development|PrintString "殴る蹴る" true true "(R=1.000000,G=0.375163,B=0.000000,A=1.000000)")
  (Development|PrintString "Delayを5.0に設定" true true "(R=1.000000,G=0.000000,B=0.129005,A=1.000000)")
  (Variables|Default|SetisAttack true)
  (return))

(fn SetIsSlime
  (params (isSlime :type Boolean))
  (Variables|Default|SetisSlime isSlime)
  (return))

(fn Damage
  (params (damage :type Float%20%28single-precision%29) (damageElem :type testElem%20Enum) (finalAttackActor :type Actor%20Object%20Reference))
  (Variables|Default|SetfinalAttackActor finalAttackActor)
  (Variables|Default|SetisDamage true)
  (bind _bairitu (CallFunction|GetAttackBairitu damageElem (Variables|Status|GetZokusei)))
  (LocalVariables|Setダメージ倍率 _bairitu)
  (bind _output_get (Variables|Status|SetHP (- (Variables|Status|GetHP) (* damage (LocalVariables|Getダメージ倍率)))))
  (if (<= _output_get 0.0)
    (if (Variables|Default|GetisSlime)
      _
      (else
        (bind _outactors (Actor|GetAllActorsOfClass "/Game/BluePrints/BattleActors/WaveMgr.WaveMgr_C"))
        (Math|Integer|DecrementInt (Variables|/Game/BluePrints/BattleActors/WaveMgr.WaveMgr_C|GetliveEnemyCnt (Utilities|Array|Get(acopy) _outactors))
          (:%20%20
            _))))
    (Actor|DestroyActor)
    (return true)
    (else
      (return false))))

(fn SetTargetActor
  (bind _self self)
  (bind _attackcol (Variables|Default|GetattackCol))
  (bind _returnvalue (AI|GetBlackboard _self))
  (bind _overlappingactors (Collision|GetOverlappingActors _attackcol "BattleActor_C" :!class /Script/Engine.PrimitiveComponent))
  (if (== (Variables|Default|GettargetActor) 0)
    (AI|Components|Blackboard|SetValueasBool _returnvalue (LocalVariables|GetBBKey_IsFight) false)
    (bind _array_element (Utilities|Array|ForEachLoopwithBreak _overlappingactors :!label _label)
      (:LoopBody
        (bind _asbattle_actor (Utilities|Casting|CastToBattleActor _array_element))
        (if (<= (Transformation|GetDistanceTo _asbattle_actor) 2e+03)
          (if (ScalableFloat|GetValueasBool (AI|GetBlackboard _asbattle_actor) (LocalVariables|GetBBKey_IsFight))
            (bind _result (Math|Integer|IncrementInt (LocalVariables|Getスルー回数))
              (:%20%20
                (if (or (>= _result 3) (>= _result (Utilities|Array|Length _overlappingactors)))
                  (if (Variables|Default|GetisSlime) :!label _label_2
                    (if (Components|ComponentHasTag (Variables|/Script/Engine.Character|GetCapsuleComponent _asbattle_actor) "Enemy")
                      (Variables|Default|SettargetActor _asbattle_actor :!label _label_3)
                      (goto _label Break))
                    (elif (Components|ComponentHasTag (Variables|/Script/Engine.Character|GetCapsuleComponent _asbattle_actor) "Slime")
                      (goto _label_3))))))
            (else
              (goto _label_2)))))
      (:Completed
        (return)))
    (else
      (AI|Components|Blackboard|SetValueasBool _returnvalue (LocalVariables|GetBBKey_IsFight) true)
      (return))))

(fn SetZokusei
  (params (Zokusei :type testElem%20Enum))
  (bind _mesh (Variables|Character|GetMesh))
  (bind _output_get (Variables|Status|SetZokusei Zokusei))
  (switch Utilities|FlowControl|Switch|SwitchontestElem _output_get
    (:NewEnumerator0
      (Rendering|Material|SetMaterial _mesh 0 "/Game/Texture/guu.guu"))
    (:NewEnumerator1
      (Rendering|Material|SetMaterial _mesh 0 "/Game/Texture/choki.choki"))
    (:NewEnumerator2
      (Rendering|Material|SetMaterial _mesh 0 "/Game/Texture/paa.paa")))
  (return))

(fn SetStatus
  (params (Status :type Str%20Battle%20Actor%20State%20Table%20Structure) (isSlime :type Boolean))
  (bind (_hp _zokusei _atdelay _walkspeed _slimetype _ap) (Utilities|Struct|BreakStr_BattleActorStateTable Status))
  (bind _mesh (Variables|Character|GetMesh))
  (bind _mesh_2 (Variables|Character|GetMesh))
  (for _array_element (Utilities|Array|MakeArray (Utilities|String|ToString(Float) _hp) (Utilities|String|EnumtoString _zokusei) (Utilities|String|ToString(Float) _atdelay) (Utilities|String|ToString(Float) _walkspeed) (Utilities|String|EnumtoString _slimetype) (Utilities|String|ToString(Float) _ap))
    (Development|PrintString _array_element true true "(R=1.000000,G=0.057227,B=0.000000,A=1.000000)" 5e+01))
  (Variables|Default|SetisSlime isSlime)
  (Variables|Status|SetHP _hp)
  (bind _output_get (Variables|Status|SetZokusei _zokusei))
  (Variables|Status|SetAP _ap)
  (Variables|Status|SetanimWaitTime _atdelay)
  (Variables|/Script/Engine.CharacterMovementComponent|SetMaxWalkSpeed (Variables|Character|GetCharacterMovement) _walkspeed)
  ;[1 1 1] デバッグ用にここで色付
  (switch Utilities|FlowControl|Switch|SwitchontestElem _output_get
    (:NewEnumerator0
      (Rendering|Material|SetMaterial _mesh_2 0 "/Game/Texture/guu.guu"))
    (:NewEnumerator1
      (Rendering|Material|SetMaterial _mesh_2 0 "/Game/Texture/choki.choki"))
    (:NewEnumerator2
      (Rendering|Material|SetMaterial _mesh_2 0 "/Game/Texture/paa.paa")))
  (if (Variables|Default|GetisSlime)
    (bind _output_get_2 (Variables|Status|SetslimeType _slimetype))
    (switch Utilities|FlowControl|Switch|SwitchonSlimeType _output_get_2
      (:NewEnumerator1
        (Class|SkinnedMeshComponent|SetSkeletalMesh _mesh "/Game/Model/Slime/normal/slaim_attack.slaim_attack"))
      (:NewEnumerator2
        (Class|SkinnedMeshComponent|SetSkeletalMesh _mesh "/Game/Model/Slime/sword/slime_sword-walk.slime_sword-walk"))
      (:NewEnumerator3
        (Class|SkinnedMeshComponent|SetSkeletalMesh _mesh "/Game/Model/Slime/armor/slime_armor_walk.slime_armor_walk"))))
  (return (Math|Conversions|ToInteger(Byte) (Variables|Status|GetslimeType))))