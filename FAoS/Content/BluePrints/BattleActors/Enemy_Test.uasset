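; Test enemy battle actor, flagged as non-slime, that attacks the slime side and drops a small gear item when destroyed.
; Attack plays an explosion on AttackCol, then adds the unique owners of overlapping components to an Actors list, which is never cleared here.
; It damages SlimeCreater actors in that list and stops at the first Slime-tagged Slime_Zako, which takes elemental damage.
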(event `self.ReceiveBeginPlay`
  (`parent.ReceiveBeginPlay`)
  (`self.setIsSlime` false))

(event `self.ReceiveDestroyed`
  (bind (_returnvalue_x _returnvalue_y) (`KismetMathLibrary.BreakVector` (`self.K2_GetActorLocation`)))
  (`|SpawnActorFromClass` "/Game/BluePrints/dropItem.dropItem_C" (`KismetMathLibrary.MakeTransform` (`KismetMathLibrary.MakeVector` _returnvalue_x _returnvalue_y) (struct) (0.3 0.3 0.3)) "Undefined" "OverrideRootScale" null "グー歯車"))

(event `self.Attack`
  (bind _actors (`self.actors`))
  (`GameplayStatics.SpawnEmitterAttached` "/Game/StarterContent/Particles/P_Explosion.P_Explosion" (`self.attackCol`))
  (`|ExecutionSequence`
    (:`then_0`
      (for _array_element (`PrimitiveComponent.GetOverlappingComponents` (`self.attackCol`))
        (bind _returnvalue (`ActorComponent.GetOwner` _array_element))
        (if (not (`KismetArrayLibrary.Array_Contains` _actors _returnvalue))
          (`KismetArrayLibrary.Array_Add` _actors _returnvalue))))
    (:`then_1`
      (for _array_element_2 (`self.actors`)
        (bind _asslime_creater (cast `/Game/BluePrints/SlimeCreater` _array_element_2)
          (:`then`
            (`/Game/BluePrints/SlimeCreater.Damaged` _asslime_creater 1.0))
          (:`CastFailed`
            (bind _asbattle_actor (cast `/Game/BluePrints/BattleActors/BattleActor` _array_element_2))))
        (if (`ActorComponent.ComponentHasTag` (`Character.CapsuleComponent` _asbattle_actor) "Slime")
          (set `self.isAttack` true)
          (bind _asslime_zako (cast `/Game/BluePrints/BattleActors/Slime_Zako` _array_element_2))
          (`self.Damage` _asslime_zako 1.0 (`self.Zokusei`)))))))

(fn `UserConstructionScript`
  (`parent.UserConstructionScript`))