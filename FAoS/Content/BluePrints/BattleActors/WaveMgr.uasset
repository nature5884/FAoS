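; Battle wave manager that spawns enemy waves and handles the level-clear sequence.
; The spawn table's row count sets the wave limit; when no enemies remain, Tick asks Enemy_SpawnMgr for the next wave, toggling enemy-AI flags around delays.
; After the final wave, it blends once to ClearCam's clear sprite, then opens GameLevel.
; CamSwitch is called around spawns but does nothing, as its outside/player camera blend logic is disconnected.
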(event `self.ReceiveBeginPlay`
  (bind _outactors (`GameplayStatics.GetAllActorsOfClass` "/Game/BluePrints/BattleActors/OutSideView.OutSideView_C"))
  (set `self.outSideCam` (`KismetArrayLibrary.Array_Get` _outactors))
  (bind _outactors_2 (`GameplayStatics.GetAllActorsOfClass` "/Game/BluePrints/PlayerCam.PlayerCam_C"))
  (set `self.playerCam` (`KismetArrayLibrary.Array_Get` _outactors_2))
  (`|ExecutionSequence`
    (:`then_0`
      (bind _outrownames (`DataTableFunctionLibrary.GetDataTableRowNames` "/Game/BluePrints/BattleActors/SpawnTable/SpawnTable.SpawnTable"))
      (set `self.waveMax` (`KismetArrayLibrary.Array_Length` _outrownames)))
    (:`then_1`
      (bind _outactors_3 (`GameplayStatics.GetAllActorsOfClass` "/Game/BluePrints/BattleActors/Enemy_SpawnMgr.Enemy_SpawnMgr_C"))
      (set `self.slimeSpawnMgr` (`KismetArrayLibrary.Array_Get` _outactors_3))
      (set `self.isAppear` true)
      (`self.CamSwitch`)
      (`KismetSystemLibrary.Delay` (`self.blrndTime`))
      (`self.appear`)
      (set `self.isAppear` false)
      (`KismetSystemLibrary.Delay` (`self.blrndTime`))
      (`self.CamSwitch`)
      (set `self.runEnemyAI_OK` true)
      (set `self.tickOK` true))))

(event `self.ReceiveTick`
  (params (DeltaSeconds :type "Float (single-precision)"))
  (if (`self.isAppear`)
    _
    (elif (<= (`self.liveEnemyCnt`) 0)
      (if (< (`self.waveCnt`) (- (`self.waveMax`) 1))
        (set `self.runEnemyAI_OK` false)
        (set `self.isAppear` true)
        (`self.CamSwitch`)
        (`KismetSystemLibrary.Delay` (`self.blrndTime`))
        (`self.appear`)
        (set `self.tickOK` false)
        (set `self.isAppear` false)
        (`KismetSystemLibrary.Delay` (`self.blrndTime`))
        (set `self.runEnemyAI_OK` true)
        (`self.CamSwitch`)
        (set `self.tickOK` false)
        (else
          (`/Engine/EditorBlueprintResources/StandardMacros.DoOnce` false
            (:`Completed`
              (bind _outactors (`GameplayStatics.GetAllActorsOfClass` "/Game/BluePrints/ClearCam.ClearCam_C"))
              (bind _item (`KismetArrayLibrary.Array_Get` _outactors))
              (bind _papersprite (`/Game/BluePrints/ClearCam.PaperSprite` _item))
              (`SceneComponent.SetVisibility` _papersprite true false)
              (`PaperSpriteComponent.SetSprite` _papersprite "/Game/Model/factory_clear2_Sprite.factory_clear2_Sprite")
              (`PlayerController.SetViewTargetWithBlend` (`GameplayStatics.GetPlayerController` 0) _item 1.0 "VTBlend_Cubic" 0.0 false)
              (`KismetSystemLibrary.Delay` 5.0)
              (`GameplayStatics.OpenLevel` "GameLevel"))))))))

(fn `appear`
  (bind (_nextwavecnt _enemycnt) (`/Game/BluePrints/BattleActors/Enemy_SpawnMgr.SpawnEnemys` (`self.slimeSpawnMgr`) (`self.waveCnt`)))
  (set `self.waveCnt` _nextwavecnt)
  (set `self.liveEnemyCnt` _enemycnt)
  (return))

(fn `CamSwitch`
  (return))

(fn `UserConstructionScript`)