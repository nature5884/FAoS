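; Slime_Zako is a slime battle actor that deals damage to enemies.
; On BeginPlay it runs the parent logic and flags itself as a slime.
; Its Attack event scans components overlapping AttackCol for the Enemy tag, casts their owners to Enemy_Test and calls Damage with a fixed amount and element.
; Damage is applied per tagged component rather than per actor.
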(event `self.ReceiveBeginPlay`
  (`parent.ReceiveBeginPlay`)
  (`self.setIsSlime` true))

(event `self.ReceiveTick`
  (params (DeltaSeconds :type "Float (single-precision)")))

(event `self.Attack`
  (for _array_element (`PrimitiveComponent.GetOverlappingComponents` (`self.attackCol`))
    (if (`ActorComponent.ComponentHasTag` _array_element "Enemy")
      (bind _asenemy_test (cast `/Game/BluePrints/BattleActors/Enemy_Test` (`ActorComponent.GetOwner` _array_element)))
      (`self.Damage` _asenemy_test 1.0 "NewEnumerator0"))))

(fn `UserConstructionScript`
  (`parent.UserConstructionScript`))