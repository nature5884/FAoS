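; Factory object Blueprint that wears down over time, breaks, and can be repaired.
; Tick lowers HP by a fixed per-frame rate without delta time, then calls Crash at zero to set the broken flag and reset repair progress.
; Repair adds progress per call but is not called within this Blueprint; once Tick sees full progress while broken, RepairFinish restores partial HP and clears the flag.
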(event `self.ReceiveTick`
  (params (DeltaSeconds :type "Float (single-precision)"))
  (bind _hp (`self.HP`))
  (if (>= _hp 0.0)
    (bind _output_get (set `self.HP` (- _hp (`self.HP減少率`)))))
  (if (<= _output_get 0.0)
    (if (`self.isCrash`)
      (if (>= (`self.repair%`) 100.0)
        (set `self.repair%` 100.0)
        (`self.RepairFinish`))
      (else
        (set `self.HP` 0.0)
        (`self.Crash`)))))

(fn `Crash`
  (`KismetSystemLibrary.PrintString` "Crash")
  (set `self.repair%` 0.0)
  (set `self.isCrash` true)
  (return))

(fn `Repair`
  (bind _repair_ (`self.repair%`))
  (`KismetSystemLibrary.PrintString` (`KismetStringLibrary.Conv_DoubleToString` _repair_))
  (set `self.repair%` (+ _repair_ (`self.repair力`)))
  (return))

(fn `RepairFinish`
  (set `self.HP` 50.0)
  (set `self.repair%` 0.0)
  (set `self.isCrash` false)
  (return))

(fn `UserConstructionScript`)