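; Factory door Blueprint that penalizes a SlimeCreater actor whenever the door is destroyed.
; On BeginPlay it caches the first SlimeCreater found in the level as Creator.
; Each Tick calls the parent and sets IsCrash from whether MyLife is at or below zero.
; A DoOnce deducts a fixed amount from Creator's Life on breaking and re-arms while MyLife is above zero.
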(event `self.ReceiveBeginPlay`
  (bind _outactors (`GameplayStatics.GetAllActorsOfClass` "/Game/BluePrints/SlimeCreater.SlimeCreater_C"))
  (set `self.creator` (`KismetArrayLibrary.Array_Get` _outactors)))

(event `self.ReceiveTick`
  (params (DeltaSeconds :type "Float (single-precision)"))
  (bind _creator (`self.creator`))
  (`parent.ReceiveTick` 0.0)
  (if (<= (`self.myLife`) 0.0)
    (set `self.isCrash` true)
    (`/Engine/EditorBlueprintResources/StandardMacros.DoOnce` false :!label _label
      (:`Completed`
        (set `/Game/BluePrints/SlimeCreater.life` (- (`/Game/BluePrints/SlimeCreater.life` _creator) 5.0) _creator)))
    (else
      (set `self.isCrash` false)
      (goto _label :!via `Reset`))))

(fn `UserConstructionScript`
  (`parent.UserConstructionScript`))