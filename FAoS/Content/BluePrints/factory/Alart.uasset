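; Factory alarm lamp actor whose emissive state, spotlight color and rotation follow the IsLightting flag.
; BeginPlay and ChangeMat create a dynamic material on the lamp mesh's second slot and set its AlarmState scalar from the flag.
; The spotlight takes its color from a material vector parameter selected by the flag.
; While lit, Tick spins the Arrow component's yaw at a frame-rate-independent speed; a spotlight visibility toggle is left unwired.
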(event `self.ReceiveBeginPlay`
  (bind _returnvalue (+ 0 1))
  (bind _factorylamp (`self.FactoryLamp`))
  (`|ExecutionSequence` :!label _label
    (:`then_0`
      ;[1 1 1] マテリアルインスタンスの作成
      (bind _returnvalue_2 (`PrimitiveComponent.CreateDynamicMaterialInstance` _factorylamp _returnvalue (`PrimitiveComponent.GetMaterial` _factorylamp _returnvalue)))
      (set `self.LampMeshMaterial` _returnvalue_2))
    (:`then_1`
      ;[1 1 1] エミッシブの選択
      (`MeshComponent.SetScalarParameterValueOnMaterials` (`self.FactoryLamp`) "AlarmState" (`KismetMathLibrary.Conv_BoolToDouble` (`self.isLightting`))))
    (:`then_2`
      (bind _returnvalue_3 (`MaterialInstanceDynamic.K2_GetVectorParameterValue` (`self.LampMeshMaterial`) (`KismetArrayLibrary.Array_Get` (`self.parameterName`) (`KismetMathLibrary.Conv_BoolToInt` (`self.isLightting`)))))
      (`LightComponent.SetLightColor` (`self.SpotLight`) _returnvalue_3 true))))

(event `ChangeMat`
  (goto _label))

(event `self.ReceiveTick`
  (params (DeltaSeconds :type "Float (single-precision)"))
  (if (`self.isLightting`)
    (`SceneComponent.K2_SetRelativeRotation` (`self.Arrow`) (`KismetMathLibrary.MakeRotator` (.roll (`SceneComponent.RelativeRotation` (`self.Arrow`))) (.pitch (`SceneComponent.RelativeRotation` (`self.Arrow`))) (+ (.yaw (`SceneComponent.RelativeRotation` (`self.Arrow`))) (* 350.0 DeltaSeconds))) false false)))

(fn `UserConstructionScript`)