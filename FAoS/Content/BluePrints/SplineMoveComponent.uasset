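; SplineMoveComponent is an actor component that moves and rotates its owner along an assigned spline at a set speed.
; Each tick it advances a travelled distance, applies the spline's location and rotation, then checks for arrival.
; On arrival it either reverses direction for ping-pong motion, wraps the overshoot when looping, or disables its tick.
; Helper functions assign the spline, adjust the distance, force an immediate move and pause by toggling tick.
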(event EventBeginPlay)

(event EventTick
  (params (DeltaSeconds :type Float%20%28single-precision%29))
  ;[1 1 1] 移動量を更新
  (Variables|Default|SetmoveDistance (+ (Variables|Default|GetmoveDistance) (* DeltaSeconds (Variables|Default|Getspeed))))
  (CallFunction|ForceMove) ; オーナーを移動
  (if (CallFunction|IsArrived)
    (if (Variables|Default|Getreturn) ; 戻るかどうか
      (if (and (not (Variables|Default|Getloop)) (<= (Variables|Default|GetmoveDistance) 0.0)) ; 到達したのはループしない始端か
        (Components|Tick|SetComponentTickEnabled false) ; 移動終了
        (else
          ;[1 1 1] 進行方向を逆に
          (Variables|Default|Setspeed (* (Variables|Default|Getspeed) -1.0))
          (Variables|Default|Setreverse (not (Variables|Default|Getreverse)))))
      (elif (Variables|Default|Getloop) ; ループするかどうか
        (Variables|Default|SetmoveDistance (- (Variables|Default|GetmoveDistance) (CallFunction|GetSplineLength))) ; 超過分の移動量を消す
        (else
          (Components|Tick|SetComponentTickEnabled false) ; 移動終了
        )))))

(fn SetSpline
  (params (NewSpline :type My%20Spline%20Actor%20Object%20Reference))
  (Variables|Default|SetSpline NewSpline)
  (Variables|Default|SetmoveDistance 0.0))

(fn IsArrived
  (if (Variables|Default|Getreverse)
    (LocalVariables|SetlocalArrived (<= (Variables|Default|GetmoveDistance) 0.0))
    (else
      (LocalVariables|SetlocalArrived (Default|IsArrived (Variables|Default|GetSpline) (Variables|Default|GetmoveDistance)))))
  (return (LocalVariables|GetlocalArrived)))

(fn GetSplineLength
  (return (Spline|GetSplineLength (Variables|/Game/BluePrints/MySplineActor.MySplineActor_C|GetSpline (Variables|Default|GetSpline)))))

(fn SetMoveDistance
  (params (NewDistance :type Float%20%28single-precision%29))
  (Variables|Default|SetmoveDistance NewDistance))

(fn AddMoveDistance
  (params (AddDistance :type Float%20%28single-precision%29))
  (CallFunction|SetMoveDistance (+ AddDistance (Variables|Default|GetmoveDistance))))

(fn ForceMove
  (bind _spline (Variables|Default|GetSpline))
  (bind _movedistance (Variables|Default|GetmoveDistance))
  (bind _loop (Variables|Default|Getloop))
  (bind _return (Variables|Default|Getreturn))
  (bind _returnvalue (not _return))
  (bind _returnvalue_2 (and _loop _returnvalue))
  (bind (_location _direction _rotation) (Default|GetCurrentLocationandRotation _spline _movedistance _returnvalue_2))
  (Transformation|SetActorLocationAndRotation (Components|GetOwner) _location _rotation))

(fn Pause
  (params (IsPause :type Boolean))
  (Components|Tick|SetComponentTickEnabled (not IsPause)))

(fn SetSplineandMove
  (params (NewSpline :type My%20Spline%20Actor%20Object%20Reference) (NewSpeed :type Float%20%28single-precision%29) (StartForceMove :type Boolean))
  (Variables|Default|SetSpline NewSpline)
  (Variables|Default|Setspeed NewSpeed)
  (Variables|Default|SetmoveDistance 0.0)
  (if StartForceMove
    (CallFunction|ForceMove)))