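; Spline actor that serves as a path, exposing distance-based queries for whatever moves along it.
; GetCurrentLocationAndRotation returns world-space location, direction and rotation at a given distance, wrapping it by modulo of the spline length when Loop is set.
; IsArrived reports whether a distance has reached the spline's end, and GetSplineLength exposes the total length.
; The event graph and construction script are empty, so the actor moves nothing itself.
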(event EventBeginPlay)

(event EventActorBeginOverlap
  (params (OtherActor :type Actor%20Object%20Reference)))

(event EventTick
  (params (DeltaSeconds :type Float%20%28single-precision%29)))

(fn ConstructionScript)

(fn IsArrived
  (params (Length :type Float%20%28single-precision%29))
  (return (>= Length (Spline|GetSplineLength (Variables|Default|GetSpline)))))

(fn GetSplineLength
  (return (Spline|GetSplineLength (Variables|Default|GetSpline))))

(fn GetCurrentLocationandRotation
  (params (Length :type Float%20%28single-precision%29) (loop :type Boolean))
  (bind _spline (Variables|Default|GetSpline))
  (if loop
    (bind _length (CallFunction|GetSplineLength))
    (LocalVariables|SetLocalLength (Math|Float|%(Float) Length _length))
    (else
      (LocalVariables|SetLocalLength Length)))
  (return (Spline|GetLocationatDistanceAlongSpline _spline (LocalVariables|GetLocalLength) "World") (Spline|GetDirectionatDistanceAlongSpline _spline (LocalVariables|GetLocalLength) "World") (Spline|GetRotationatDistanceAlongSpline _spline (LocalVariables|GetLocalLength) "World")))