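; Slime factory actor that turns queued orders from the player character into AI slimes and has its own life value.
; StackCreate, bound to MyCharacter at BeginPlay, queues count, type and kind; Tick works through the queue, spawning Slime_Zako on a timer with stats and anim class.
; Tick also shows a screen-projected "press E to add materials" prompt while the possessing player overlaps ThrowPoint.
; Depleted life only prints a factory-destroyed message.
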(event `self.ReceiveBeginPlay`
  (bind _asmy_character (cast `/Game/BluePrints/MyCharacter` (`GameplayStatics.GetPlayerPawn` 0)))
  (add `/Game/BluePrints/MyCharacter.SlimeCreate` _asmy_character (delegate `StackCreate`)))

(event `StackCreate`
  (params (NewParam :type "/Game/BluePrints/sozai/ItemTypeStructure Structure"))
  (`KismetArrayLibrary.Array_Add` (`self.ItemType`) (make `/Game/BluePrints/sozai/ItemTypeStructure` `NewParam_生成数_5_13B98CB44FEE2F45198CF49FE88DC7BC` `NewParam_タイプ_8_A1BB91A248550689571F43B041FFEC80` `NewParam_種別_12_A9CDB4224F793D4986A2E4AE2381427C`)))

(event `self.ReceiveTick`
  (params (DeltaSeconds :type "Float (single-precision)"))
  (bind _stacknum (`self.stackNum`))
  (bind _itemtype (`self.ItemType`))
  (bind (`_item_生成数` `_item_タイプ` `_item_種別`) (break `/Game/BluePrints/sozai/ItemTypeStructure` (`KismetArrayLibrary.Array_Get` _itemtype)))
  (bind _returnvalue_location (`KismetMathLibrary.BreakTransform` (`SceneComponent.K2_GetComponentToWorld` (`self.spawnPoint`))))
  (set `self.frameCnt` DeltaSeconds)
  (`|ExecutionSequence`
    (:`then_0`
      (if (> (`KismetArrayLibrary.Array_Length` _itemtype) 0)
        (`|ExecutionSequence`
          (:`then_0`
            (`/Engine/EditorBlueprintResources/StandardMacros.DoOnce` false :!label _label
              (:`Completed`
                (set `self.stackNum` `_item_生成数`)
                (set `self.Type` `_item_タイプ`)
                (set `self.MyKind` `_item_種別`)
                (set `self.startCreate` true))))
          (:`then_1`
            (if (and (`self.startCreate`) (> (`self.stackNum`) 0))
              (bind _output_get (set `self.timer` (- (`self.timer`) (`self.frameCnt`))))
              (if (<= _output_get 0.0)
                (bind _returnvalue (`AIBlueprintHelperLibrary.SpawnAIFromClass` "/Game/BluePrints/BattleActors/Slime_Zako.Slime_Zako_C" "/Game/BluePrints/BattleActors/AI/Slime/BT_Slime.BT_Slime" _returnvalue_location))
                (bind _asbattle_actor (cast `/Game/BluePrints/BattleActors/BattleActor` _returnvalue))
                (bind _type (`/Game/BluePrints/BattleActors/BattleActor.SetStatus` _asbattle_actor (make `/Game/BluePrints/BattleActors/Str_EnemyStateTable` 15.0 (`self.Type`) 1.0 70.0) true (`self.MyKind`)))
                (`SkeletalMeshComponent.SetAnimInstanceClass` (`Character.Mesh` _asbattle_actor) (`KismetArrayLibrary.Array_Get` (`self.AnimInst`) _type))
                (bind _result (`/Engine/EditorBlueprintResources/StandardMacros.DecrementInt` _stacknum)
                  (:`  `
                    (set `self.stackNum` _result)
                    (set `self.timer` 3.0)
                    (if (== _stacknum 0)
                      (set `self.startCreate` false)
                      (`KismetArrayLibrary.Array_Remove` (`self.ItemType`))
                      (goto _label :!via `Reset`))))))))))
    (:`then_1`
      (bind _outactors (`GameplayStatics.GetAllActorsOfClass` "/Game/BluePrints/TestHUD.TestHUD_C"))
      (bind _asmy_character (cast `/Game/BluePrints/MyCharacter` (`GameplayStatics.GetPlayerPawn` 0)))
      (if (`/Game/BluePrints/MyCharacter.isPossess` _asmy_character)
        (if (`self.canThrow`)
          (bind _e_buttontext (`/Game/BluePrints/TestWidget.E_ButtonText` (`/Game/BluePrints/TestHUD.MyWidget` (`KismetArrayLibrary.Array_Get` _outactors))))
          (`Widget.SetVisibility` _e_buttontext "Visible")
          (`Widget.SetRenderTranslation` _e_buttontext (`GameplayStatics.ProjectWorldToScreen` (`GameplayStatics.GetPlayerController` 0) (`SceneComponent.K2_GetComponentLocation` (`self.textSetter`))))
          (`MultiLineEditableTextBox.SetText` _e_buttontext "Eボタンで \n素材を投入！")
          (else
            (`Widget.SetVisibility` _e_buttontext "Hidden" :!label _label_2)))
        (else
          (goto _label_2))))))

(event `self.throwPoint.OnComponentBeginOverlap`
  (params (OtherActor :type "Actor Object Reference") (OtherComp :type "PrimitiveComponent Object Reference") (OtherBodyIndex :type Integer) (bFromSweep :type Boolean) (SweepResult :type "HitResult Structure (by ref)"))
  (if (== OtherActor (`GameplayStatics.GetPlayerPawn` 0))
    (set `self.canThrow` true)))

(event `self.throwPoint.OnComponentEndOverlap`
  (params (OtherActor :type "Actor Object Reference") (OtherComp :type "PrimitiveComponent Object Reference") (OtherBodyIndex :type Integer))
  (if (== OtherActor (`GameplayStatics.GetPlayerPawn` 0))
    (set `self.canThrow` false)))

(fn `Damaged`
  (params (damageNum :type "Float (double-precision)"))
  (bind _life (`self.life`))
  (set `self.life` (- _life damageNum))
  (if (<= _life 0.0)
    (`self.GameOver`)))

(fn `GameOver`
  (`KismetSystemLibrary.PrintString` "工場爆破"))

(fn `UserConstructionScript`)