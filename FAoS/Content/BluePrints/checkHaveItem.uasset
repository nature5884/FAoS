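; Trigger actor that checks whether the player carries an item and, if so, takes over their movement.
; Overlapping CollisionComponent with the item disables player input and fires CallPlayerMove.
; The Sphere trigger fires CallPlayerMove again after a one-second delay.
; Sphere1 restores input and clears IsHaveItem, reusing the character cast from the first overlap.
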(event `self.CollisionComponent.OnComponentBeginOverlap`
  (params (OtherActor :type "Actor Object Reference") (OtherComp :type "PrimitiveComponent Object Reference") (OtherBodyIndex :type Integer) (bFromSweep :type Boolean) (SweepResult :type "HitResult Structure (by ref)"))
  (bind _returnvalue (`GameplayStatics.GetPlayerPawn` 0))
  (bind _asmy_character (cast `/Game/BluePrints/MyCharacter` _returnvalue))
  (if (and (== OtherActor _returnvalue) (`/Game/BluePrints/MyCharacter.isHaveItem` _asmy_character))
    (`self.DisableInput` _returnvalue (`GameplayStatics.GetPlayerController` 0))
    (`self.PlayerMove`)))

(event `self.Sphere.OnComponentBeginOverlap`
  (params (OtherActor :type "Actor Object Reference") (OtherComp :type "PrimitiveComponent Object Reference") (OtherBodyIndex :type Integer) (bFromSweep :type Boolean) (SweepResult :type "HitResult Structure (by ref)"))
  (if (== OtherActor (`GameplayStatics.GetPlayerPawn` 0))
    (`KismetSystemLibrary.Delay` 1.0)
    (`self.PlayerMove`)))

(event `self.Sphere1.OnComponentBeginOverlap`
  (params (OtherActor :type "Actor Object Reference") (OtherComp :type "PrimitiveComponent Object Reference") (OtherBodyIndex :type Integer) (bFromSweep :type Boolean) (SweepResult :type "HitResult Structure (by ref)"))
  (bind _returnvalue (`GameplayStatics.GetPlayerPawn` 0))
  (if (== OtherActor _returnvalue)
    (`self.EnableInput` _returnvalue (`GameplayStatics.GetPlayerController` 0))
    (set `/Game/BluePrints/MyCharacter.isHaveItem` false (stale `self.CollisionComponent.OnComponentBeginOverlap` _asmy_character))))

(fn `UserConstructionScript`)