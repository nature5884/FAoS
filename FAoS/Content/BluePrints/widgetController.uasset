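; Widget controller actor that shows an animated wave-number announcement on the HUD whenever a new wave appears.
; On BeginPlay it looks up the TestHUD actor, whose MyWidget holds the wave text and animation.
; Tick polls the first WaveMgr's IsAppear flag, using a DoOnce to increment the wave count, set the text and play the animation.
; When the animation stops, Tick hides the text, clears the flag and resets the DoOnce.
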(event `self.ReceiveBeginPlay`
  (if (not (!= (`self.testHUD`) null))
    (bind _outactors (`GameplayStatics.GetAllActorsOfClass` "/Game/BluePrints/TestHUD.TestHUD_C"))
    (set `self.testHUD` (`KismetArrayLibrary.Array_Get` _outactors))))

(event `self.ReceiveTick`
  (params (DeltaSeconds :type "Float (single-precision)"))
  (bind _wavecount (`self.waveCount`))
  (bind _wavechange (`self.waveChange`))
  (bind _mywidget (`/Game/BluePrints/TestHUD.MyWidget` (`self.testHUD`)))
  (bind _wavetextbox (`/Game/BluePrints/TestWidget.waveTextBox` _mywidget))
  (bind _wavetextanim (`/Game/BluePrints/TestWidget.waveTextAnim` _mywidget))
  (bind _returnvalue (`UserWidget.IsAnimationPlaying` _mywidget _wavetextanim))
  (`|ExecutionSequence`
    (:`then_0`
      (bind _outactors (`GameplayStatics.GetAllActorsOfClass` "/Game/BluePrints/BattleActors/WaveMgr.WaveMgr_C"))
      (if (`/Game/BluePrints/BattleActors/WaveMgr.isAppear` (`KismetArrayLibrary.Array_Get` _outactors))
        (set `self.waveChange` true)))
    (:`then_1`
      (if _wavechange
        (`/Engine/EditorBlueprintResources/StandardMacros.DoOnce` false :!label _label
          (:`Completed`
            (bind _result (`/Engine/EditorBlueprintResources/StandardMacros.IncrementInt` _wavecount)
              (:`  `
                (set `self.waveCount` _result)
                (`Widget.SetVisibility` _wavetextbox "Visible")
                (`Widget.SetVisibility` _mywidget "Visible")
                (`UserWidget.SetPositionInViewport` _mywidget (0.0 0.0) true)
                (`MultiLineEditableTextBox.SetText` _wavetextbox (`KismetTextLibrary.Conv_StringToText` (`KismetStringLibrary.Concat_StrStr` (`self.S_wave`) (`KismetStringLibrary.Conv_IntToString` _wavecount))))
                (`UserWidget.PlayAnimation` _mywidget _wavetextanim 0.0 1 "Forward")
                (if (not _returnvalue)
                  (`Widget.SetVisibility` _wavetextbox "Hidden" :!label _label_2)
                  (set `self.waveChange` false)
                  (goto _label :!via `Reset`))))))))
    (:`then_2`
      (if (and _wavechange (not _returnvalue))
        (goto _label_2)))))

(fn `UserConstructionScript`)